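; BP_Rail is a spline-based rail actor that builds its meshes in the Construction Script.
; It adds one SplineMeshComponent per segment of MySpline, using RailStartMesh for the first, RailEndMesh for the last and RailMidMesh between.
; The SetStartAndEnd node that would fit each piece to its segment's locations and tangents is not wired into execution, so the pieces do not follow the spline.
; The Event Graph has no active logic.
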(fn `UserConstructionScript`
  (bind _returnvalue (- (`SplineComponent.GetNumberOfSplinePoints` (`self.MySpline`)) 2))
  (for _index (range (+ _returnvalue 1))
    (bind _returnvalue_2 (`AddComponent|NODE_AddSplineMeshComponent-0`))
    (if (== _index 0)
      (`StaticMeshComponent.SetStaticMesh` _returnvalue_2 (`self.RailStartMesh`))
      (elif (== _index _returnvalue)
        (`StaticMeshComponent.SetStaticMesh` _returnvalue_2 (`self.RailEndMesh`))
        (else
          (`StaticMeshComponent.SetStaticMesh` _returnvalue_2 (`self.RailMidMesh`)))))))